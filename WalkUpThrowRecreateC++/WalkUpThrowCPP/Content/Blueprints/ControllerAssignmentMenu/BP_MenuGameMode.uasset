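; Game mode for the controller assignment menu that registers two joining players and then starts gameplay.
; On each join it plays a sound, tells the WB_MenuWidget reached through BP_MenuHUD, and stores the pad index for player 1 or 2 in WUT_GameInstance.
; It counts joins and opens the Gameplay level once the count reaches two.
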(event `self.OnPlayerJoined`
  (params (PlayerIndex :type Integer) (PadIndex :type Integer))
  (`AudioComponent.Play` (`self.Sfx`) 0.0)
  (bind _asbp_menu_hud (castclass `/Game/Blueprints/ControllerAssignmentMenu/BP_MenuHUD` (`self.HUDClass`)))
  (bind _returnvalue (`GameplayStatics.GetActorOfClass` _asbp_menu_hud))
  (bind _aswb_menu_widget (cast `/Game/Blueprints/ControllerAssignmentMenu/WB_MenuWidget` (`WUT_MenuHUD.GetMenuWidget` _returnvalue)))
  (`/Game/Blueprints/ControllerAssignmentMenu/WB_MenuWidget.PlayerJoined` _aswb_menu_widget PlayerIndex)
  (bind _aswut_game_instance (cast `WUT_GameInstance` (`GameplayStatics.GetGameInstance`)))
  (switch `int` PlayerIndex
    (:`1`
      (set `WUT_GameInstance.Player1PadIndex` PadIndex _aswut_game_instance))
    (:`2`
      (set `WUT_GameInstance.Player2PadIndex` PadIndex _aswut_game_instance)))
  (bind _output_get (set `self.PlayerCount` (+ (`self.PlayerCount`) 1)))
  (if (>= _output_get 2)
    (`GameplayStatics.OpenLevel` "Gameplay")))

(fn `UserConstructionScript`)