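; Player character for a two-player sprite fighting game, with IsPlayer2 selecting input mapping, tint and block direction.
; Enhanced Input drives movement, attack, throw and blocking, including hold-back blocking, through state flags and animation node jumps.
; Per-frame events reshape the leg hurtbox, while overlap checks apply damage or grab the opponent.
; Finished Hadokens and throws cost the loser one health, triggering a reset or winner call.
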(event `LoadControls`
  ; Instantiate Control
  (bind _asplayer_controller (cast `PlayerController` (`self.GetController`) :!label _label))
  (bind _returnvalue (pcsubsystem `EnhancedInputLocalPlayerSubsystem` _asplayer_controller))
  (`/Engine/EditorBlueprintResources/StandardMacros.IsValid` _returnvalue
    (:`Is Valid`
      (if (`self.IsPlayer2`)
        (`EnhancedInputSubsystemInterface.AddMappingContext` _returnvalue "/Game/Controls/IMC_Player2.IMC_Player2" 0 (struct))
        (`self.EnableInput` null)
        (else
          (`EnhancedInputSubsystemInterface.AddMappingContext` _returnvalue "/Game/Controls/IMC_Player1.IMC_Player1" 0 (struct))))
      ; Set Up Speed
      (set `self.playerSpeed` (`CharacterMovementComponent.MaxWalkSpeed` (`self.CharacterMovement`)))
      ; Enabled Collision
      (`PrimitiveComponent.SetCollisionEnabled` (`self.LegHurtBox`) "NoCollision"))))

(event `self.ReceiveBeginPlay`
  ; Instantiate Control
  (goto _label))

(event `EnhancedInput|/Game/Controls/Throw_IA`
  (params (ActionValue :type Boolean) (ElapsedSeconds :type "Float (double-precision)") (TriggeredSeconds :type "Float (double-precision)") (InputAction :type "InputAction Object Reference" :default "/Game/Controls/Throw_IA.Throw_IA"))
  (:`Started`
    (set `self.IsTryThrowing` true)))

(event `EnhancedInput|/Game/Controls/Attack_IA`
  (params (ActionValue :type Boolean) (ElapsedSeconds :type "Float (double-precision)") (TriggeredSeconds :type "Float (double-precision)") (InputAction :type "InputAction Object Reference" :default "/Game/Controls/Attack_IA.Attack_IA"))
  (bind _charactermovement (`self.CharacterMovement`))
  (bind _animinstance (`PaperZDAnimationComponent.AnimInstance` (`self.AnimationComponent`)))
  (:`Started`
    ; Attack
    (if (`/Game/Blueprints/PlayerCharacter_BP.IsHurt` (`self.Opponent`))
      (`PaperZDAnimInstance.JumpToNode` _animinstance "HitConfirm" "None")
      (set `self.IsHitConfirm` true)
      (elif (not (`self.IsHitConfirm`))
        (`/Engine/EditorBlueprintResources/StandardMacros.DoOnce` false :!label _label_2
          (:`Completed`
            (if (`self.IsBlocking`)
              (set `self.IsBlocking` false))
            (set `CharacterMovementComponent.MaxWalkSpeed` 0.0 _charactermovement)
            (`PaperZDAnimInstance.JumpToNode` _animinstance "Attack" "None")
            (set `self.IsAttack` true)
            (`KismetSystemLibrary.Delay` (`PaperFlipbookComponent.GetFlipbookLength` (`self.Sprite`)))
            (set `CharacterMovementComponent.MaxWalkSpeed` (`self.playerSpeed`) _charactermovement)
            (goto _label_2 :!via `Reset`))))))
  (:`Completed`
    (set `self.IsAttack` false)))

(event `self.ReceiveAnyDamage`
  (params (Damage :type "Float (single-precision)") (DamageType :type "DamageType Object Reference") (InstigatedBy :type "Controller Object Reference") (DamageCauser :type "Actor Object Reference"))
  (bind _charactermovement (`self.CharacterMovement`))
  ; OnAttackHit
  (if (`self.IsToBeBlock`)
    (set `self.IsBlocking` true)
    (elif (`self.IsBlocking`)
      _
      (elif (not (`self.IsHurt`))
        (set `self.IsHurt` true)
        (`PaperZDAnimInstance.JumpToNode` (`PaperZDAnimationComponent.AnimInstance` (`self.AnimationComponent`)) "Hurt" "None")
        (set `CharacterMovementComponent.MaxWalkSpeed` 0.0 _charactermovement)
        (`KismetSystemLibrary.RetriggerableDelay` (`PaperFlipbookComponent.GetFlipbookLength` (`self.Sprite`)))
        (set `CharacterMovementComponent.MaxWalkSpeed` (`self.playerSpeed`) _charactermovement)))))

(event `BlockPlayer2`
  ; Block
  (set `self.IsBlocking` true :!label _label_3)
  (set `CharacterMovementComponent.MaxWalkSpeed` 0.0 (`self.CharacterMovement`)))

(event `EnhancedInput|/Game/Controls/Block_IA`
  (params (ActionValue :type Boolean) (ElapsedSeconds :type "Float (double-precision)") (TriggeredSeconds :type "Float (double-precision)") (InputAction :type "InputAction Object Reference" :default "/Game/Controls/Block_IA.Block_IA"))
  ; Block
  (:`Triggered`
    (goto _label_3))
  (:`Completed`
    (set `self.IsBlocking` false :!label _label_4)
    (set `CharacterMovementComponent.MaxWalkSpeed` (`self.playerSpeed`) (`self.CharacterMovement`))))

(event `OnHadokenFinished`
  (bind _opponent (`self.Opponent`))
  (if (not (`/Game/Blueprints/PlayerCharacter_BP.IsLose` _opponent))
    (set `/Game/Blueprints/PlayerCharacter_BP.IsLose` true _opponent)
    (`self.LoseFn` _opponent)
    (bind _health (`self.LoseHealth` _opponent))
    (if (> _health 0.0)
      (`self.Reset`))))

(event `StopBlockingPlayer2`
  ; Block
  (goto _label_4))

(event `EnhancedInput|/Game/Controls/Move_IA`
  (params (ActionValue :type "Float (double-precision)") (ElapsedSeconds :type "Float (double-precision)") (TriggeredSeconds :type "Float (double-precision)") (InputAction :type "InputAction Object Reference" :default "/Game/Controls/Move_IA.Move_IA"))
  (bind _returnvalue (> ActionValue 0.0))
  ; Move Action (Player 1)
  (:`Triggered`
    (`self.AddMovementInput` (1.0 0.0 0.0) ActionValue)
    (if (`self.IsPlayer2`)
      (if _returnvalue
        (set `self.IsToBeBlock` true :!label _label_5))
      (elif (not _returnvalue)
        (goto _label_5))))
  (:`Completed`
    (set `self.IsToBeBlock` false)))

(event `self.ReceiveTick`
  (params (DeltaSeconds :type "Float (single-precision)"))
  (if (`/Game/Blueprints/PlayerCharacter_BP.IsAttack` (`self.Opponent`))
    _
    (elif (`self.IsToBeBlock`)
      (`KismetSystemLibrary.Delay` 0.2)
      (set `self.IsBlocking` false))))

(event `Attack`
  ; Attack
  (for _array_element (`PrimitiveComponent.GetOverlappingActors` (`self.AttackBox`) null)
    (if (!= _array_element self)
      (`GameplayStatics.ApplyDamage` _array_element (`self.baseDamage`)))))

(event `Frame1LegExtend`
  (bind _leghurtbox (`self.LegHurtBox`))
  ; Frame1LegCollisionBoxHandler
  (`PrimitiveComponent.SetCollisionEnabled` _leghurtbox "QueryOnly")
  (`SceneComponent.K2_SetRelativeLocation` _leghurtbox (58.5 0.0 -40.0) false false)
  (`SceneComponent.SetWorldScale3D` _leghurtbox (0.4125 1.0 1.0)))

(event `Frame2LegExtend`
  (bind _leghurtbox (`self.LegHurtBox`))
  ; Frame2LegCollisionBoxHandler
  (`PrimitiveComponent.SetCollisionEnabled` _leghurtbox "QueryOnly")
  (`SceneComponent.K2_SetRelativeLocation` _leghurtbox (71.0 0.0 -40.0) false false)
  (`SceneComponent.SetWorldScale3D` _leghurtbox (0.87 1.0 1.0)))

(event `Throw`
  (bind _opponent (`self.Opponent`))
  (for _array_element (`PrimitiveComponent.GetOverlappingActors` (`self.ThrowHitBox`) null)
    (if (!= _array_element self)
      (`self.ExecuteThrow`)
      (set `/Game/Blueprints/PlayerCharacter_BP.IsBeingThrown` true _opponent)
      (`self.DisableInput` _opponent null)
      (`CharacterMovementComponent.SetMovementMode` (`Character.CharacterMovement` _opponent) "MOVE_Flying" 0)
      (`self.K2_SetActorLocation` _opponent (`SceneComponent.K2_GetComponentLocation` (`self.ThrowHitBox`)) false false)
      (`self.GetHurt` _opponent))))

(event `Frame3LegExtend`
  (bind _leghurtbox (`self.LegHurtBox`))
  ; Frame3LegCollisionBoxHandler
  (`PrimitiveComponent.SetCollisionEnabled` _leghurtbox "QueryOnly")
  (`SceneComponent.K2_SetRelativeLocation` _leghurtbox (100.0 0.0 -40.0) false false)
  (`SceneComponent.SetWorldScale3D` _leghurtbox (1.75 1.0 1.0)))

(event `OnAttackEnd`
  ; OnAttackEnd
  (`PrimitiveComponent.SetCollisionEnabled` (`self.LegHurtBox`) "NoCollision"))

(event `ReleaseThrow`
  (bind _opponent (`self.Opponent`))
  (`CharacterMovementComponent.SetMovementMode` (`Character.CharacterMovement` _opponent) "MOVE_Walking" 0)
  (`self.BeingThrown` _opponent)
  (`self.Reset`))

(event `IsDoneHurt`
  ; OnHurtEnd
  (set `self.IsHurt` false))

(event `OnLoseEnd`
  (bind _opponent (`self.Opponent`))
  (if (not (`/Game/Blueprints/PlayerCharacter_BP.IsWin` _opponent))
    (set `/Game/Blueprints/PlayerCharacter_BP.IsWin` true _opponent)
    (`self.OnWinBegin` _opponent)))

(event `OnWinBegin`
  (`PaperZDAnimInstance.JumpToNode` (`PaperZDAnimationComponent.AnimInstance` (`self.AnimationComponent`)) "YouWin" "None"))

(event `OnTryThrowFinish`
  (set `self.IsTryThrowing` false))

(fn `BeingThrown`
  (set `self.IsBeingThrown` true)
  (if (not (`self.IsLose`))
    (set `self.IsLose` true)
    (`self.LoseFn`)
    (bind _health (`self.LoseHealth`))
    (if (> _health 0.0)
      _)))

(fn `ExecuteThrow`
  (set `self.IsThrowing` true))

(fn `GetHurt`
  (`PaperZDAnimInstance.JumpToNode` (`PaperZDAnimationComponent.AnimInstance` (`self.AnimationComponent`)) "BeingThrown" "None"))

(fn `LoseFn`
  (`PaperZDAnimInstance.JumpToNode` (`PaperZDAnimationComponent.AnimInstance` (`self.AnimationComponent`)) "Lose" "None")
  (`self.LaunchCharacter` (350.0 0.0 350.0))
  (`self.DisableInput` (`GameplayStatics.GetPlayerPawn` 0) null)
  (`self.DisableInput` (`GameplayStatics.GetPlayerPawn` 1) null))

(fn `LoseHealth`
  (returns (Health :type "Float (double-precision)"))
  (bind _output_get (set `self.health` (- (`self.health`) 1.0)))
  (if (<= _output_get 0.0)
    (set `self.health` 0.0)
    (`self.WhoWon`)
    (else
      (`self.UpdateHealth`)))
  (return (`self.health`)))

(fn `ResetState`
  (`self.EnableInput` (`GameplayStatics.GetPlayerPawn` 0) null)
  (`self.EnableInput` (`GameplayStatics.GetPlayerPawn` 1) null)
  (set `self.IsWin` false)
  (set `self.IsLose` false)
  (set `self.IsTryThrowing` false)
  (set `self.IsThrowing` false)
  (set `self.IsBeingThrown` false)
  (set `self.IsHurt` false)
  (set `self.IsToBeBlock` false)
  (set `self.IsAttack` false)
  (set `self.IsHitConfirm` false)
  (`PaperZDAnimInstance.JumpToNode` (`PaperZDAnimationComponent.AnimInstance` (`self.AnimationComponent`)) "Idle" "None"))

(fn `UserConstructionScript`
  (if (`self.IsPlayer2`)
    (`PaperFlipbookComponent.SetSpriteColor` (`self.Sprite`) (struct :`R` 1.0 :`G` 0.276042 :`B` 0.575308 :`A` 1.0))))