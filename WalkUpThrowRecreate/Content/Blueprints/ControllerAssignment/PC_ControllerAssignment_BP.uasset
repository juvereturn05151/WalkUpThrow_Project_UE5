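; Player controller for controller assignment, letting a local player flag itself as ready through Enhanced Input.
; On BeginPlay it adds the controller-assignment mapping context to the local player subsystem of the controller at its own controller ID plus one.
; The Ready input action sets the IsReady flag through SetPlayerReady.
; Debug prints report the ID, mapping setup result and ready state, using the same offset lookup for the name.
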(event `self.ReceiveBeginPlay`
  (bind _returnvalue (+ (`GameplayStatics.GetPlayerControllerID` null) 1))
  (bind _returnvalue_2 (pcsubsystem `EnhancedInputLocalPlayerSubsystem` (`GameplayStatics.GetPlayerController` _returnvalue)))
  (`KismetSystemLibrary.PrintString` (`KismetStringLibrary.Conv_IntToString` _returnvalue))
  (`/Engine/EditorBlueprintResources/StandardMacros.IsValid` _returnvalue_2
    (:`Is Valid`
      (`EnhancedInputSubsystemInterface.AddMappingContext` _returnvalue_2 "/Game/Controls/IMC_ControllerAssignment.IMC_ControllerAssignment" 0 (struct))
      (`KismetSystemLibrary.PrintString` "Init Mapping Context Successfully"))
    (:`Is Not Valid`
      (`KismetSystemLibrary.PrintString` "Fail"))))

(event `EnhancedInput|/Game/Controls/Ready_IA`
  (params (ActionValue :type Boolean) (ElapsedSeconds :type "Float (double-precision)") (TriggeredSeconds :type "Float (double-precision)") (InputAction :type "InputAction Object Reference" :default "/Game/Controls/Ready_IA.Ready_IA"))
  (:`Triggered`
    (`self.SetPlayerReady` true)
    (`KismetSystemLibrary.PrintString` (`KismetStringLibrary.Concat_StrStr` (`KismetSystemLibrary.GetDisplayName` (`GameplayStatics.GetPlayerController` (+ (`GameplayStatics.GetPlayerControllerID` null) 1))) "IsReady"))))

(fn `SetPlayerReady`
  (params (_ready :type Boolean))
  (set `self.bIsReady` _ready))

(fn `UserConstructionScript`)