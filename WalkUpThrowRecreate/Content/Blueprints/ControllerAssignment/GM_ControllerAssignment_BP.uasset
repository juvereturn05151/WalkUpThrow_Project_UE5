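; Game mode for the controller assignment screen, setting up the UI and up to two local players.
; On BeginPlay it creates the assignment widget, then creates a second local player if more than one input device is connected.
; It caches both player controllers as PC_ControllerAssignment_BP and passes them to the widget through SetPlayer, printing a debug failure message if either cast fails.
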(event `self.ReceiveBeginPlay`
  (`self.Create_ControllerAssignment_UI`)
  (`self.Create_Player2_IfConnected`)
  (`self.AssignPlayerControllers_ControllerAssignment`)
  (`self.AssignPlayerControllersToWB`))

(fn `AssignPlayerControllers_ControllerAssignment`
  (bind _aspc_controller_assignment_bp (cast `/Game/Blueprints/ControllerAssignment/PC_ControllerAssignment_BP` (`GameplayStatics.GetPlayerController` 0))
    (:`then`
      (set `self.PlayerController1` _aspc_controller_assignment_bp)
      (bind _aspc_controller_assignment_bp_2 (cast `/Game/Blueprints/ControllerAssignment/PC_ControllerAssignment_BP` (`GameplayStatics.GetPlayerController` 1))
        (:`then`
          (set `self.PlayerController2` _aspc_controller_assignment_bp_2))
        (:`CastFailed`
          (`KismetSystemLibrary.PrintString` "Fail" :!label _label))))
    (:`CastFailed`
      (goto _label))))

(fn `AssignPlayerControllersToWB`
  (`/Game/Blueprints/ControllerAssignment/WB_ControllerAssignment.Set_Player` (`self.ControllerAssignment_WB`) (`self.PlayerController1`) (`self.PlayerController2`)))

(fn `Create_ControllerAssignment_UI`
  (bind _returnvalue (`|CreateWidget` "/Game/Blueprints/ControllerAssignment/WB_ControllerAssignment.WB_ControllerAssignment_C"))
  (`UserWidget.AddToViewport` _returnvalue 0)
  (set `self.ControllerAssignment_WB` _returnvalue))

(fn `Create_Player2_IfConnected`
  (bind _outinputdevices (`InputDeviceLibrary.GetAllConnectedInputDevices`))
  (if (> (`KismetArrayLibrary.Array_Length` _outinputdevices) 1)
    (bind _returnvalue (`GameplayStatics.CreatePlayer` 1))
    (`KismetSystemLibrary.PrintString` (`KismetStringLibrary.Concat_StrStr` "Create Player:" (`KismetSystemLibrary.GetDisplayName` _returnvalue)))))

(fn `UserConstructionScript`)