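; Game mode for a local two-player fighting game that runs the round flow and restarts it on reset.
; BeginPlay spawns and possesses both characters as mutual opponents, views through the MainCamera-tagged actor and creates the health bar widget.
; Character events drive health bar updates, winner checks and delayed resets to the spawn transforms.
; Tick advances Ready, Fight and Gameplay phases through one-second Delays, keeping input disabled until Gameplay.
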(event `self.ReceiveBeginPlay`
  (`self.SetUpPlayers`)
  (`self.SetUpWidgets`)
  (`self.DoReady`)
  (add `/Game/Blueprints/PlayerCharacter_BP.UpdateHealth` (`self.Player2Ref`) (delegate `UpdateHealthbar`))
  (add `/Game/Blueprints/PlayerCharacter_BP.UpdateHealth` (`self.Player1Ref`) (delegate `UpdateHealthbar`))
  (`/Game/UI/HealthBar_WB.UpdateHealthbar` (`self.gameUIref`) :!label _label)
  (add `/Game/Blueprints/PlayerCharacter_BP.WhoWon` (`self.Player1Ref`) (delegate `CheckWhoWon`))
  (add `/Game/Blueprints/PlayerCharacter_BP.WhoWon` (`self.Player2Ref`) (delegate `CheckWhoWon`))
  (add `/Game/Blueprints/PlayerCharacter_BP.Reset` (`self.Player1Ref`) (delegate `ResetEvent`))
  (add `/Game/Blueprints/PlayerCharacter_BP.Reset` (`self.Player2Ref`) (delegate `ResetEvent`)))

(event `UpdateHealthbar`
  (goto _label))

(event `ResetEvent`
  (`KismetSystemLibrary.Delay` 2.0)
  (`self.ResetGame`)
  (`self.DoReady`))

(event `CheckWhoWon`
  (`/Game/UI/HealthBar_WB.CheckWhoWin` (`self.gameUIref`)))

(event `self.ReceiveTick`
  (params (DeltaSeconds :type "Float (single-precision)"))
  (if (== (`self.CurrentPhase`) 0)
    (`KismetSystemLibrary.Delay` 1.0)
    (`self.DoFight`)
    (elif (== (`self.CurrentPhase`) 1)
      (`KismetSystemLibrary.Delay` 1.0)
      (`self.DoGameplay`)
      (elif (== (`self.CurrentPhase`) 3)
        _))))

(fn `DoFight`
  (set `self.CurrentPhase` "NewEnumerator1")
  (`/Game/UI/HealthBar_WB.Fight` (`self.gameUIref`)))

(fn `DoGameplay`
  (set `self.CurrentPhase` "NewEnumerator2")
  (`/Game/UI/HealthBar_WB.Gameplay` (`self.gameUIref`))
  (`self.EnableInput` (`GameplayStatics.GetPlayerPawn` 0) null)
  (`self.EnableInput` (`GameplayStatics.GetPlayerPawn` 1) null))

(fn `DoReady`
  (set `self.CurrentPhase` "NewEnumerator0")
  (`/Game/UI/HealthBar_WB.Ready` (`self.gameUIref`))
  (`self.DisableInput` (`GameplayStatics.GetPlayerPawn` 0) null)
  (`self.DisableInput` (`GameplayStatics.GetPlayerPawn` 1) null))

(fn `ResetGame`
  (`self.K2_SetActorTransform` (`self.Player1Ref`) (`self.Character1Transformation`) false false)
  (`self.K2_SetActorTransform` (`self.Player2Ref`) (`self.Character2Transformation`) false false)
  (`/Game/Blueprints/PlayerCharacter_BP.ResetState` (`self.Player1Ref`))
  (`/Game/Blueprints/PlayerCharacter_BP.ResetState` (`self.Player2Ref`))
  (set `self.CurrentPhase` "NewEnumerator0"))

(fn `SetUpPlayers`
  (bind _returnvalue (`GameplayStatics.GetPlayerController` 0))
  (bind _player1ref (`self.Player1Ref`))
  (bind _player2ref (`self.Player2Ref`))
  (bind _returnvalue_2 (`|SpawnActorFromClass` "/Game/Blueprints/PlayerCharacter_BP.PlayerCharacter_BP_C" (`self.Character1Transformation`) "Undefined" "MultiplyWithRoot" null false null))
  (bind _output_get (set `self.Player1Ref` _returnvalue_2))
  (`Controller.Possess` _returnvalue _output_get)
  (bind _outactors (`GameplayStatics.GetAllActorsWithTag` "MainCamera"))
  (`PlayerController.SetViewTargetWithBlend` _returnvalue (`|GetArrayItem` _outactors) 0.0 "VTBlend_Linear" 0.0 false)
  (`/Game/Blueprints/PlayerCharacter_BP.LoadControls` (`self.Player1Ref`))
  (`GameplayStatics.CreatePlayer` 1)
  (bind _returnvalue_3 (`|SpawnActorFromClass` "/Game/Blueprints/PlayerCharacter_BP.PlayerCharacter_BP_C" (`self.Character2Transformation`) "Undefined" "MultiplyWithRoot" null true null))
  (set `self.Player2Ref` _returnvalue_3)
  (`Controller.Possess` (`GameplayStatics.GetPlayerController` 1) _returnvalue_3)
  (`/Game/Blueprints/PlayerCharacter_BP.LoadControls` _returnvalue_3)
  (set `/Game/Blueprints/PlayerCharacter_BP.Opponent` _player2ref _player1ref)
  (set `/Game/Blueprints/PlayerCharacter_BP.Opponent` _player1ref _player2ref))

(fn `SetUpWidgets`
  (bind _returnvalue (`|CreateWidget` "/Game/UI/HealthBar_WB.HealthBar_WB_C" null (`self.Player1Ref`) (`self.Player2Ref`)))
  (bind _output_get (set `self.gameUIref` _returnvalue))
  (`UserWidget.AddToViewport` _output_get 0))

(fn `UserConstructionScript`)